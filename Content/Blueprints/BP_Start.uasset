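; BP_Start is the starting piece of a procedural corridor chain, seeding the corridors and their paintings at BeginPlay.
; It spawns a linked BP_Corridor ahead of itself, extends the chain through each corridor's CreateNext, then has all corridors spawn paintings.
; A looping timer destroys the actor once the player is out of range.
; Tick updates two point lights' offset positions from their parents and stored start locations.
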(event `self.ReceiveBeginPlay`
  (`KismetSystemLibrary.K2_SetTimerDelegate` (delegate `CheckPlayerDistance`) 1.0 true)
  ;[1 1 1] Set light starting positions
  (set `self.Light1StartPosition` (`SceneComponent.K2_GetComponentLocation` (`self.PointLight1`)))
  (set `self.Light2StartPosition` (`SceneComponent.K2_GetComponentLocation` (`self.PointLight2`)))
  (`self.SpawnCorridors`))

(event `CheckPlayerDistance`
  (bind _withinrange (`/Game/Blueprints/BP_Util.WithinRangeOfPlayer` self 600.0))
  (if (not _withinrange)
    (`self.K2_DestroyActor`)))

(event `self.ReceiveTick`
  (params (DeltaSeconds :type "Float (single-precision)"))
  (`/Game/Blueprints/BP_Util.UpdateOffsetPosition` (`self.Light1Parent`) (`self.PointLight1`) (`self.Light1StartPosition`))
  (`/Game/Blueprints/BP_Util.UpdateOffsetPosition` (`self.Light2Parent`) (`self.PointLight2`) (`self.Light2StartPosition`)))

(fn `SpawnCorridors`
  (locals (Corridors :type "Array of Actor Object Reference"))
  (bind (_returnvalue_location _returnvalue_rotation _returnvalue_scale) (`KismetMathLibrary.BreakTransform` (`self.GetTransform`)))
  ;[1 1 1] Create first corridor
  (bind _returnvalue (`|SpawnActorFromClass` "/Game/Blueprints/BP_Corridor.BP_Corridor_C" (`KismetMathLibrary.MakeTransform` (+ _returnvalue_location (600.0 0.0 0.0)) _returnvalue_rotation _returnvalue_scale) "Undefined" "MultiplyWithRoot" null null))
  (set `/Game/Blueprints/BP_Corridor.PreviousCorridor` self _returnvalue)
  (bind _output_get (set `self.Corridor` _returnvalue))
  (`KismetArrayLibrary.Array_Add` (`local.Corridors`) _output_get)
  ;[1 1 1] Create additional corridors
  (for _ (range 1 (+ (`self.InitialCorridorCount`) 1))
    (bind _asbp_corridor (cast `/Game/Blueprints/BP_Corridor` (`self.Corridor`)))
    (bind _next (`/Game/Blueprints/BP_Corridor.CreateNext` _asbp_corridor))
    (bind _output_get_2 (set `self.Corridor` _next))
    (`KismetArrayLibrary.Array_Add` (`local.Corridors`) _output_get_2))
  ;[1 1 1] Spawn Paintings
  (for _array_element (`local.Corridors`)
    (bind _asbp_corridor_2 (cast `/Game/Blueprints/BP_Corridor` _array_element))
    (`/Game/Blueprints/BP_Corridor.SpawnPaintings` _asbp_corridor_2)))

(fn `UserConstructionScript`)