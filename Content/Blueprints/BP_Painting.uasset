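; BP_Painting is an actor that displays a rendered snapshot of the scene on its Mirror component.
; SetSceneCapture stores a supplied capture actor, creates a canvas render target, feeds it to a dynamic M_Mirror material and calls CaptureScene once.
; A looping timer from BeginPlay checks player range and destroys both the capture actor and the painting when the check fails.
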(event `self.ReceiveBeginPlay`
  (`KismetSystemLibrary.K2_SetTimerDelegate` (delegate `CheckPlayerDistance`) 1.0 true))

(event `CheckPlayerDistance`
  (bind _withinrange (`/Game/Blueprints/BP_Util.WithinRangeOfPlayer` self 600.0))
  (if (not _withinrange)
    (`self.K2_DestroyActor` (`self.Capture`))
    (`self.K2_DestroyActor`)))

(fn `SetSceneCapture`
  (params (SceneCapture :type "/Game/Blueprints/BP_PaintingCapture Object Reference"))
  (bind _capturecomponent2d (`SceneCapture2D.CaptureComponent2D` (`self.Capture`)))
  (set `self.Capture` SceneCapture)
  (bind _returnvalue (`CanvasRenderTarget2D.CreateCanvasRenderTarget2D` "/Script/Engine.CanvasRenderTarget2D" (`self.RenderTargetWidth`) (`self.RenderTargetHeight`)))
  (bind _returnvalue_2 (`PrimitiveComponent.CreateDynamicMaterialInstance` (`self.Mirror`) 0 "/Game/Materials/M_Mirror.M_Mirror" "Test"))
  (`MaterialInstanceDynamic.SetTextureParameterValue` _returnvalue_2 "RenderTarget" _returnvalue)
  (set `SceneCaptureComponent2D.TextureTarget` _returnvalue _capturecomponent2d)
  (`SceneCaptureComponent2D.CaptureScene` _capturecomponent2d))

(fn `UserConstructionScript`)