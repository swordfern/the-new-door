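; Shared utility functions for procedurally building a first-person world of corridors, intersections, paintings and mirrors.
; Corridors spawn only within player range, becoming intersections at grid-spaced positions, flipped by player-relative facing, with helpers linking neighbors.
; Paintings spawn at random points in boxes, each fed by a randomly rotated scene capture; mirrors spawn when the game mode allows.
; A camera-relative sideways offset, growing quadratically with distance, curves component positions.
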(fn `CreateOffsetActor`
  (params (GameMode :type "/Game/FirstPerson/Blueprints/BP_FirstPersonGameMode Object Reference") (Parent :type "Actor Object Reference") (Offset :type "Vector Structure") (Class :type "Actor Class Reference") (TargetSize :type "Float (double-precision)") (Rotation :type "Rotator Structure"))
  (returns (Actor :type "Actor Object Reference"))
  (bind (_returnvalue_location _returnvalue_rotation) (`KismetMathLibrary.BreakTransform` (`Actor.GetTransform` Parent)))
  (bind _location (`self.GetRelativeLocation` Parent Offset (`local.__WorldContext`)))
  (bind _withinrange (`self.LocationWithinRangeOfPlayer` _location TargetSize (`local.__WorldContext`)))
  (if _withinrange
    (`KismetSystemLibrary.PrintString` null "Creating corridor")
    (bind _actor (`/Game/FirstPerson/Blueprints/BP_FirstPersonGameMode.SpawnActor` GameMode Class (`KismetMathLibrary.MakeTransform` _location (`KismetMathLibrary.ComposeRotators` _returnvalue_rotation Rotation))))
    (return _actor)))

(fn `GetRelativeLocation`
  (params (Target :type "Actor Object Reference") (Offset :type "Vector Structure"))
  (returns (Location :type "Vector Structure"))
  (bind (_returnvalue_location _returnvalue_rotation) (`KismetMathLibrary.BreakTransform` (`Actor.GetTransform` Target)))
  (return (+ _returnvalue_location (`KismetMathLibrary.GreaterGreater_VectorRotator` Offset _returnvalue_rotation))))

(fn `InverseLerp`
  (params (A :type "Float (double-precision)") (B :type "Float (double-precision)") (V :type "Float (double-precision)"))
  (returns (InverseLerp :type "Float (double-precision)"))
  (return (/ (- V A) (- B A))))

(fn `LocationWithinRangeOfPlayer`
  (params (TargetLocation :type "Vector Structure") (TargetSize :type "Float (double-precision)"))
  (returns (WithinRange :type Boolean))
  (bind _asbp_first_person_game_mode (cast `/Game/FirstPerson/Blueprints/BP_FirstPersonGameMode` (`GameplayStatics.GetGameMode` (`local.__WorldContext`))))
  (bind _returnvalue (`GameplayStatics.GetActorOfClass` null "/Game/FirstPerson/Blueprints/BP_FirstPersonCharacter.BP_FirstPersonCharacter_C"))
  (`/Engine/EditorBlueprintResources/StandardMacros.IsValid` _returnvalue
    (:`Is Valid`
      (bind _returnvalue_location (`KismetMathLibrary.BreakTransform` (`Actor.GetTransform` _returnvalue)))
      (return (< (`KismetMathLibrary.Vector_DistanceSquared` _returnvalue_location TargetLocation) (`KismetMathLibrary.Square` (+ (`/Game/FirstPerson/Blueprints/BP_FirstPersonGameMode.PlayerRange` _asbp_first_person_game_mode) TargetSize)))))
    (:`Is Not Valid`
      (`KismetSystemLibrary.PrintString` (`local.__WorldContext`) "Unable to find player character"))))

(fn `SetNextCorridorParent`
  (params (Next :type "Object Object Reference") (Parent :type "Actor Object Reference"))
  (`/Engine/EditorBlueprintResources/StandardMacros.IsValid` Next
    (:`Is Valid`
      (bind _asbp_corridor (cast `/Game/Blueprints/BP_Corridor` Next)
        (:`then`
          (set `/Game/Blueprints/BP_Corridor.PreviousCorridor` Parent _asbp_corridor))
        (:`CastFailed`
          (bind _asbp_intersection (cast `/Game/Blueprints/BP_Intersection` Next))
          (set `/Game/Blueprints/BP_Intersection.PreviousCorridor` Parent _asbp_intersection))))))

(fn `SetPreviousCorridorParent`
  (params (Previous :type "Object Object Reference") (Parent :type "Actor Object Reference"))
  (`/Engine/EditorBlueprintResources/StandardMacros.IsValid` Previous
    (:`Is Valid`
      (bind _asbp_corridor (cast `/Game/Blueprints/BP_Corridor` Previous)
        (:`then`
          (set `/Game/Blueprints/BP_Corridor.NextCorridor` Parent _asbp_corridor))
        (:`CastFailed`
          (bind _asbp_intersection (cast `/Game/Blueprints/BP_Intersection` Previous))
          (set `/Game/Blueprints/BP_Intersection.NextCorridor` Parent _asbp_intersection))))))

(fn `Should Spawn Intersection`
  (params (Target :type "Actor Object Reference") (Offset :type "Vector Structure") (IntersectionDistance :type "Float (double-precision)"))
  (returns (SpawnIntersection :type Boolean))
  (bind (_returnvalue_location _returnvalue_rotation) (`KismetMathLibrary.BreakTransform` (`Actor.GetTransform` Target)))
  (bind (_returnvalue_x _returnvalue_y) (`KismetMathLibrary.BreakVector` (+ _returnvalue_location (`KismetMathLibrary.GreaterGreater_VectorRotator` Offset _returnvalue_rotation))))
  (return (and (`KismetMathLibrary.NearlyEqual_FloatFloat` (mod (`KismetMathLibrary.Conv_IntToDouble` (`KismetMathLibrary.Round` _returnvalue_x)) IntersectionDistance) 0.0 1.0) (`KismetMathLibrary.NearlyEqual_FloatFloat` (mod (`KismetMathLibrary.Conv_IntToDouble` (`KismetMathLibrary.Round` _returnvalue_y)) IntersectionDistance) 0.0 1.0))))

(fn `ShouldFlipIntersection`
  (params (Intersection :type "/Game/Blueprints/BP_Intersection Object Reference"))
  (returns (ShouldFlip :type Boolean))
  (bind _returnvalue_location (`KismetMathLibrary.BreakTransform` (`Actor.GetTransform` Intersection)))
  (bind _returnvalue (`GameplayStatics.GetActorOfClass` (`local.__WorldContext`) "/Game/FirstPerson/Blueprints/BP_FirstPersonCharacter.BP_FirstPersonCharacter_C"))
  (bind _returnvalue_location_2 (`KismetMathLibrary.BreakTransform` (`Actor.GetTransform` _returnvalue)))
  (return (< (`KismetMathLibrary.Dot_VectorVector` (`KismetMathLibrary.Vector_Normal2D` (`KismetMathLibrary.GetRightVector` (`KismetMathLibrary.Conv_VectorToRotator` (- _returnvalue_location _returnvalue_location_2)))) (`KismetMathLibrary.Vector_Normal2D` (- (`SceneComponent.K2_GetComponentLocation` (`/Game/Blueprints/BP_Intersection.Facing` Intersection)) _returnvalue_location))) 0.0)))

(fn `Spawn Painting Capture`
  (params (MinRotation :type "Rotator Structure") (MaxRotation :type "Rotator Structure") (Boxes :type "Array of BoxComponent Object Reference (by ref)"))
  (returns (PaintingCapture :type "/Game/Blueprints/Paintings/BP_PaintingCapture Object Reference"))
  (bind _actor (`self.SpawnActorInBox` "/Game/Blueprints/Paintings/BP_PaintingCapture.BP_PaintingCapture_C" Boxes))
  (bind _asbp_painting_capture (cast `/Game/Blueprints/Paintings/BP_PaintingCapture` _actor))
  (`Actor.K2_AddActorLocalRotation` _asbp_painting_capture (`KismetMathLibrary.MakeRotator` (`KismetMathLibrary.RandomFloatInRange` (.roll MinRotation) (.roll MaxRotation)) (`KismetMathLibrary.RandomFloatInRange` (.pitch MinRotation) (.pitch MaxRotation)) (`KismetMathLibrary.RandomFloatInRange` (.yaw MinRotation) (.yaw MaxRotation))) false false)
  (return _asbp_painting_capture))

(fn `SpawnActorInBox`
  (params (Class :type "Actor Class Reference") (Boxes :type "Array of BoxComponent Object Reference"))
  (returns (Actor :type "Actor Object Reference"))
  (bind _output (`|GetArrayItem` Boxes (`KismetMathLibrary.RandomIntegerInRange` 0 (- (`KismetArrayLibrary.Array_Length` Boxes) 1))))
  (bind (_origin _boxextent) (`KismetSystemLibrary.GetComponentBounds` _output))
  (bind _asbp_first_person_game_mode (cast `/Game/FirstPerson/Blueprints/BP_FirstPersonGameMode` (`GameplayStatics.GetGameMode` null)))
  (bind _actor (`/Game/FirstPerson/Blueprints/BP_FirstPersonGameMode.SpawnActor` _asbp_first_person_game_mode Class (`KismetMathLibrary.MakeTransform` (`KismetMathLibrary.RandomPointInBoundingBox` _origin _boxextent) (`SceneComponent.K2_GetComponentRotation` _output))))
  (return _actor))

(fn `SpawnPainting`
  (params (PaintingClasses :type "Array of Actor Class Reference") (Boxes :type "Array of BoxComponent Object Reference (by ref)"))
  (returns (Painting :type "/Game/Blueprints/Paintings/BP_PaintingA Object Reference"))
  (locals (SpawnedPainting :type "Actor Object Reference"))
  (while (not (`KismetSystemLibrary.IsValid` (`local.SpawnedPainting`)))
    (bind _actor (`self.SpawnActorInBox` (`|GetArrayItem` PaintingClasses (`KismetMathLibrary.RandomIntegerInRange` 0 (- (`KismetArrayLibrary.Array_Length` PaintingClasses) 1))) Boxes))
    (set `local.SpawnedPainting` _actor))
  (bind _asbp_painting_a (cast `/Game/Blueprints/Paintings/BP_PaintingA` (`local.SpawnedPainting`)))
  (return _asbp_painting_a))

(fn `SpawnPaintings`
  (params (MinPaintings :type Integer) (MaxPaintings :type Integer) (MinCaptureRotation :type "Rotator Structure") (MaxCaptureRotation :type "Rotator Structure") (Boxes :type "Array of BoxComponent Object Reference") (PaintingClasses :type "Array of /Game/Blueprints/Paintings/BP_PaintingA Class Reference"))
  (locals (Painting :type "Actor Object Reference"))
  (for _ (range 1 (+ (`KismetMathLibrary.RandomIntegerInRange` MinPaintings MaxPaintings) 1))
    (bind _paintingcapture (`self.Spawn Painting Capture` MinCaptureRotation MaxCaptureRotation Boxes))
    (bind _painting (`self.SpawnPainting` PaintingClasses Boxes))
    (`/Game/Blueprints/Paintings/BP_PaintingCapture.SetupRenderTarget` _paintingcapture (`/Game/Blueprints/Paintings/BP_PaintingA.RenderTargetWidth` _painting) (`/Game/Blueprints/Paintings/BP_PaintingA.RenderTargetHeight` _painting))
    (`/Game/Blueprints/Paintings/BP_PaintingA.SetSceneCapture` _painting _paintingcapture)))

(fn `Try Create Corridor`
  (params (ExistingCorridor :type "Actor Object Reference") (Parent :type "Actor Object Reference") (Offset :type "Vector Structure") (Rotation :type "Rotator Structure"))
  (returns (Created :type Boolean) (Corridor :type "Actor Object Reference"))
  (`/Engine/EditorBlueprintResources/StandardMacros.IsValid` ExistingCorridor
    (:`Is Valid`
      (return false null))
    (:`Is Not Valid`
      (bind _asbp_first_person_game_mode (cast `/Game/FirstPerson/Blueprints/BP_FirstPersonGameMode` (`GameplayStatics.GetGameMode` (`local.__WorldContext`))))
      (if (`self.Should Spawn Intersection` Parent Offset (`/Game/FirstPerson/Blueprints/BP_FirstPersonGameMode.IntersectionDistance` _asbp_first_person_game_mode) (`local.__WorldContext`))
        (bind _actor (`self.CreateOffsetActor` _asbp_first_person_game_mode Parent Offset "/Game/Blueprints/BP_Intersection.BP_Intersection_C" 600.0 Rotation (`local.__WorldContext`)))
        (`/Engine/EditorBlueprintResources/StandardMacros.IsValid` _actor
          (:`Is Valid`
            (bind _asbp_intersection (cast `/Game/Blueprints/BP_Intersection` _actor))
            (bind _shouldflip (`self.ShouldFlipIntersection` _asbp_intersection (`local.__WorldContext`)))
            (if _shouldflip
              (`/Game/Blueprints/BP_Intersection.Flip` _asbp_intersection))
            (return true _asbp_intersection))
          (:`Is Not Valid`
            (return false null)))
        (else
          (bind _actor_2 (`self.CreateOffsetActor` _asbp_first_person_game_mode Parent Offset "/Game/Blueprints/BP_Corridor.BP_Corridor_C" 600.0 Rotation (`local.__WorldContext`)))
          (return (`KismetSystemLibrary.IsValid` _actor_2) _actor_2))))))

(fn `TrySpawnMirror`
  (params (Parent :type "Actor Object Reference") (Boxes :type "Array of BoxComponent Object Reference"))
  (bind _returnvalue_location (`KismetMathLibrary.BreakTransform` (`Actor.GetTransform` Parent)))
  (bind _asbp_first_person_game_mode (cast `/Game/FirstPerson/Blueprints/BP_FirstPersonGameMode` (`GameplayStatics.GetGameMode` null)))
  (if (`/Game/FirstPerson/Blueprints/BP_FirstPersonGameMode.CanSpawnMirror` _asbp_first_person_game_mode _returnvalue_location)
    (`self.SpawnActorInBox` "/Game/Blueprints/BP_Mirror.BP_Mirror_C" Boxes)))

(fn `UpdateOffsetPosition`
  (params (ReferencePosition :type "SceneComponent Object Reference") (SceneComponent :type "SceneComponent Object Reference") (StartPosition :type "Vector Structure"))
  (bind _worldpositionoffset (`self.WorldPositionOffset` ReferencePosition (`local.__WorldContext`)))
  (`SceneComponent.K2_SetWorldLocation` SceneComponent (+ _worldpositionoffset StartPosition) false false))

(fn `WithinRangeOfPlayer`
  (params (Target :type "Actor Object Reference") (TargetSize :type "Float (double-precision)") (OverrideRange :type Boolean) (Range :type "Float (double-precision)"))
  (returns (WithinRange :type Boolean))
  (bind _returnvalue_location (`KismetMathLibrary.BreakTransform` (`Actor.GetTransform` Target)))
  (bind _asbp_first_person_game_mode (cast `/Game/FirstPerson/Blueprints/BP_FirstPersonGameMode` (`GameplayStatics.GetGameMode` null)))
  (bind _returnvalue (`GameplayStatics.GetActorOfClass` null "/Game/FirstPerson/Blueprints/BP_FirstPersonCharacter.BP_FirstPersonCharacter_C"))
  (`/Engine/EditorBlueprintResources/StandardMacros.IsValid` _returnvalue
    (:`Is Valid`
      (bind _returnvalue_location_2 (`KismetMathLibrary.BreakTransform` (`Actor.GetTransform` _returnvalue)))
      (return (< (`KismetMathLibrary.Vector_DistanceSquared` _returnvalue_location_2 _returnvalue_location) (`KismetMathLibrary.Square` (+ (`KismetMathLibrary.SelectFloat` Range (`/Game/FirstPerson/Blueprints/BP_FirstPersonGameMode.PlayerRange` _asbp_first_person_game_mode) OverrideRange) TargetSize)))))
    (:`Is Not Valid`
      (`KismetSystemLibrary.PrintString` (`local.__WorldContext`) "Unable to find player character"))))

(fn `WorldPositionOffset`
  (params (SceneComponent :type "SceneComponent Object Reference"))
  (returns (WorldPositionOffset :type "Vector Structure"))
  (bind _returnvalue (`SceneComponent.K2_GetComponentLocation` SceneComponent))
  (bind _returnvalue_2 (`GameplayStatics.GetActorOfClass` null "/Game/FirstPerson/Blueprints/BP_FirstPersonCharacter.BP_FirstPersonCharacter_C"))
  (bind _asbp_first_person_game_mode (cast `/Game/FirstPerson/Blueprints/BP_FirstPersonGameMode` (`GameplayStatics.GetGameMode` null)))
  (bind _returnvalue_3 (`SceneComponent.K2_GetComponentLocation` (`/Game/FirstPerson/Blueprints/BP_FirstPersonCharacter.FirstPersonCamera` _returnvalue_2)))
  (bind _returnvalue_4 (`KismetMathLibrary.Vector_Distance` _returnvalue_3 _returnvalue))
  (return (* (`KismetMathLibrary.Cross_VectorVector` (`KismetMathLibrary.Normal` (- _returnvalue _returnvalue_3)) (`KismetMathLibrary.Vector_Up`)) (`KismetMathLibrary.Lerp` 0.0 _returnvalue_4 (`self.InverseLerp` 0.0 (`/Game/FirstPerson/Blueprints/BP_FirstPersonGameMode.CurveFalloffDistance` _asbp_first_person_game_mode) _returnvalue_4)))))