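; BP_Intersection is a three-way junction piece in a procedurally spawned corridor world.
; On spawn it places random paintings in its boxes and tries to put a mirror on the big wall.
; A one-second timer creates missing next, previous and side corridors and links them while the player is near, and destroys the intersection otherwise.
; Flip rotates the geometry and switches which side the branch corridor spawns on.
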(event `self.ReceiveBeginPlay`
  (bind _box3 (`self.Box3`))
  (`KismetSystemLibrary.K2_SetTimerDelegate` (delegate `CheckPlayerDistance`) 1.0 true)
  (`/Game/Blueprints/BP_Util.SpawnPaintings` (`self.Min Paintings`) (`self.Max Paintings`) (`self.Min Capture Rotation`) (`self.Max Capture Rotation`) (`|MakeArray` (`self.Box1`) (`self.Box2`) _box3 _box3 (`self.Box4`)) (`|MakeArray` "/Game/Blueprints/Paintings/BP_PaintingAIntersection.BP_PaintingAIntersection_C" "/Game/Blueprints/Paintings/BP_PaintingBIntersection.BP_PaintingBIntersection_C" "/Game/Blueprints/Paintings/BP_PaintingCIntersection.BP_PaintingCIntersection_C" :!type "/Game/Blueprints/Paintings/BP_PaintingA Class Reference"))
  (`/Game/Blueprints/BP_Util.TrySpawnMirror` self (`|MakeArray` (`self.Box1`))) ; Mirror is less likely to collide if it only spawns on big wall
)

(event `CheckPlayerDistance`
  (bind _isflipped (`self.IsFlipped`))
  (bind _withinrange (`/Game/Blueprints/BP_Util.WithinRangeOfPlayer` self 1200.0))
  (if _withinrange
    ;[1 1 1] Next Corridor
    (bind (_created _corridor) (`/Game/Blueprints/BP_Util.Try Create Corridor` (`self.NextCorridor`) self (600.0 0.0 0.0)))
    (if _created
      (bind _output_get (set `self.NextCorridor` _corridor))
      (`/Game/Blueprints/BP_Util.SetNextCorridorParent` _output_get self))
    ;[1 1 1] Previous Corridor
    (bind (_created_2 _corridor_2) (`/Game/Blueprints/BP_Util.Try Create Corridor` (`self.PreviousCorridor`) self (-600.0 0.0 0.0)))
    (if _created_2
      (bind _output_get_2 (set `self.PreviousCorridor` _corridor_2))
      (`/Game/Blueprints/BP_Util.SetPreviousCorridorParent` _output_get_2 self))
    ;[1 1 1] Right Corridor
    (bind (_created_3 _corridor_3) (`/Game/Blueprints/BP_Util.Try Create Corridor` (`self.RightCorridor`) self (`KismetMathLibrary.SelectVector` (0.0 -600.0 0.0) (0.0 600.0 0.0) _isflipped) (`KismetMathLibrary.SelectRotator` (struct :`Yaw` -90.0) (struct :`Yaw` 90.0) _isflipped)))
    (if _created_3
      (bind _output_get_3 (set `self.RightCorridor` _corridor_3))
      (`/Game/Blueprints/BP_Util.SetNextCorridorParent` _output_get_3 self))
    (else
      (`self.K2_DestroyActor`))))

(fn `Flip`
  (`KismetSystemLibrary.PrintString` "Intersection should be flipped")
  (set `self.IsFlipped` true)
  (`SceneComponent.K2_SetRelativeRotation` (`self.Geometry`) (struct :`Yaw` 180.0) false false))

(fn `UserConstructionScript`)