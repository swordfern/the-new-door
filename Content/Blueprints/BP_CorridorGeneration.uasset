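; BP_CorridorGeneration builds a straight run of corridor pieces capped by an intersection when play begins.
; On BeginPlay it loops from 1 to Count, spawning a Corridor actor at each multiple of Size, then spawns one Intersection a step past the last.
; Spawn locations are measured from the world origin, ignoring the generator's own transform, and the construction script is empty.
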(event `self.ReceiveBeginPlay`
  (for _index (range 1 (+ (`self.Count`) 1))
    (`|SpawnActorFromClass` (`self.Corridor`) (`KismetMathLibrary.MakeTransform` (* _index (`self.Size`))) "Undefined" "MultiplyWithRoot" null null))
  (`|SpawnActorFromClass` (`self.Intersection`) (`KismetMathLibrary.MakeTransform` (* (+ (`self.Count`) 1) (`self.Size`))) "Undefined" "MultiplyWithRoot" null null))

(fn `UserConstructionScript`)