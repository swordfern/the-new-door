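; BP_Corridor is a corridor segment that extends itself endlessly around the player.
; A looping timer checks player proximity: in range, it tries to create next and previous segments offset along X, otherwise it destroys itself.
; New neighbours get linked back to their creator, forming a chain of corridors.
; It tries to spawn a mirror on BeginPlay and spawns paintings once when in range, both using two boxes.
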(event `self.ReceiveBeginPlay`
  (bind _boxes (`self.Boxes`))
  (`KismetSystemLibrary.K2_SetTimerDelegate` (delegate `CheckPlayerDistance`) 1.0 true)
  ;[1 1 1] Populate Boxes
  (`KismetArrayLibrary.Array_Add` _boxes (`self.Box1`))
  (`KismetArrayLibrary.Array_Add` _boxes (`self.Box2`))
  (`/Game/Blueprints/BP_Util.TrySpawnMirror` self (`self.Boxes`)))

(event `CheckPlayerDistance`
  (bind _withinrange (`/Game/Blueprints/BP_Util.WithinRangeOfPlayer` self 600.0))
  (if _withinrange
    (`self.CreateNext`)
    (`self.Create Previous`)
    (`self.SpawnPaintings`)
    (else
      (`self.K2_DestroyActor`))))

(fn `Create Previous`
  (returns (Previous :type "Actor Object Reference"))
  (bind (_created _corridor) (`/Game/Blueprints/BP_Util.Try Create Corridor` (`self.PreviousCorridor`) self (-600.0 0.0 0.0)))
  (if _created
    (bind _output_get (set `self.PreviousCorridor` _corridor))
    (`/Game/Blueprints/BP_Util.SetPreviousCorridorParent` _output_get self)
    (return _output_get)))

(fn `CreateNext`
  (returns (Next :type "Actor Object Reference"))
  (bind (_created _corridor) (`/Game/Blueprints/BP_Util.Try Create Corridor` (`self.NextCorridor`) self (600.0 0.0 0.0)))
  (if _created
    (bind _output_get (set `self.NextCorridor` _corridor))
    (`/Game/Blueprints/BP_Util.SetNextCorridorParent` _output_get self)
    (return _output_get)
    (else
      (return null))))

(fn `SpawnPaintings`
  (locals (Painting :type "Actor Object Reference"))
  (if (not (`self.HasSpawnedPaintings`))
    (set `self.HasSpawnedPaintings` true)
    (`/Game/Blueprints/BP_Util.SpawnPaintings` (`self.MinPaintings`) (`self.MaxPaintings`) (`self.MinCaptureRotation`) (`self.MaxCaptureRotation`) (`self.Boxes`) (`|MakeArray` "/Game/Blueprints/Paintings/BP_PaintingA.BP_PaintingA_C" "/Game/Blueprints/Paintings/BP_PaintingB.BP_PaintingB_C" "/Game/Blueprints/Paintings/BP_PaintingC.BP_PaintingC_C" :!type "/Game/Blueprints/Paintings/BP_PaintingA Class Reference"))))

(fn `UserConstructionScript`)