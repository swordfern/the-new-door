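; BP_PaintingCapture is a scene capture actor that renders a view into a render target, apparently for paintings.
; On BeginPlay it hands its CaptureComponent2D to the BPUpdateOffsetPosition helper.
; SetupRenderTarget creates a canvas render target at a given size and assigns it as the capture's texture.
; Capture updates the offset position through the helper, captures the scene on demand and flags HasCaptured.
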(event `self.ReceiveBeginPlay`
  (`/Game/Blueprints/BP_UpdateOffsetPosition.Set Scene` (`self.BP_UpdateOffsetPosition`) (`self.CaptureComponent2D`)))

(fn `Capture`
  (`/Game/Blueprints/BP_UpdateOffsetPosition.UpdateOffsetPosition` (`self.BP_UpdateOffsetPosition`))
  (`SceneCaptureComponent2D.CaptureScene` (`self.CaptureComponent2D`))
  (set `self.HasCaptured` true))

(fn `SetupRenderTarget`
  (params (RenderTargetWidth :type Integer) (RenderTargetHeight :type Integer))
  (bind _returnvalue (`CanvasRenderTarget2D.CreateCanvasRenderTarget2D` "/Script/Engine.CanvasRenderTarget2D" RenderTargetWidth RenderTargetHeight))
  (bind _output_get (set `SceneCaptureComponent2D.TextureTarget` _returnvalue (`self.CaptureComponent2D`)))
  (set `self.RenderTarget` _output_get))

(fn `UserConstructionScript`)