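; Painting actor that displays a one-time scene capture, shown only once the player has come within capture range.
; SetSceneCapture stores the paired capture actor and feeds its render target into a dynamic material on the Mirror component.
; It starts hidden; a looping timer triggers the capture and reveals it when in range, avoiding continuous capture.
; The same timer destroys both painting and capture actor when the player is too far away.
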(event `self.ReceiveBeginPlay`
  (`KismetSystemLibrary.K2_SetTimerDelegate` (delegate `CheckPlayerDistance`) 1.0 true)
  (`SceneComponent.SetVisibility` (`self.DefaultSceneRoot`) false true))

(event `CheckPlayerDistance`
  (`self.TryCaptureScene`)
  ;[1 1 1] Destroy if too far away
  (bind _withinrange (`/Game/Blueprints/BP_Util.WithinRangeOfPlayer` self 600.0))
  (if (not _withinrange)
    (`self.K2_DestroyActor` (`self.Scene Capture`))
    (`self.K2_DestroyActor`)))

(fn `SetSceneCapture`
  (params (SceneCapture :type "/Game/Blueprints/Paintings/BP_PaintingCapture Object Reference"))
  (bind _output_get (set `self.Scene Capture` SceneCapture))
  (bind _returnvalue (`PrimitiveComponent.CreateDynamicMaterialInstance` (`self.Mirror`) 0 "/Game/Materials/MI_Painting.MI_Painting" "DynamicPainting"))
  (`MaterialInstanceDynamic.SetTextureParameterValue` _returnvalue "RenderTarget" (`/Game/Blueprints/Paintings/BP_PaintingCapture.RenderTarget` _output_get))
  (`self.TryCaptureScene`))

(fn `TryCaptureScene`
  (bind _scene_capture (`self.Scene Capture`))
  (if (not (`/Game/Blueprints/Paintings/BP_PaintingCapture.HasCaptured` _scene_capture))
    (bind _withinrange (`/Game/Blueprints/BP_Util.WithinRangeOfPlayer` self 0.0 true (`self.CaptureRange`)))
    (if _withinrange
      (`/Game/Blueprints/Paintings/BP_PaintingCapture.Capture` _scene_capture)
      (`SceneComponent.SetVisibility` (`self.DefaultSceneRoot`) true true))))

(fn `UserConstructionScript`)