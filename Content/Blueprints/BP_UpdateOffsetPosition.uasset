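; Actor component that updates an offset position for a target scene component every tick, relative to a recorded start location.
; SetScene stores the target and its current world location, enables ticking and runs one update immediately.
; BeginPlay ticks only if a valid target exists.
; The offset math lives in UpdateOffsetPosition, which is not defined here.
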(event `self.ReceiveBeginPlay`
  (`self.SetComponentTickEnabled` (`KismetSystemLibrary.IsValid` (`self.SceneComponent`))))

(event `self.ReceiveTick`
  (params (DeltaSeconds :type "Float (single-precision)"))
  (`/Game/Blueprints/BP_Util.UpdateOffsetPosition` (`self.SceneComponent`) (`self.StartLocation`)))

(fn `Set Scene`
  (params (Scene :type "SceneComponent Object Reference"))
  (set `self.SceneComponent` Scene)
  (set `self.StartLocation` (`self.K2_GetComponentLocation` Scene))
  (`self.SetComponentTickEnabled` true)
  (`/Game/Blueprints/BP_Util.UpdateOffsetPosition` (`self.SceneComponent`) (`self.StartLocation`)))