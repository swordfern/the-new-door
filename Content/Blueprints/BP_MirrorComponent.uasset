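; BP_MirrorComponent drives the owning actor's SceneCaptureComponent2D to act as a mirror view that responds to the player.
; On BeginPlay it finds that capture component and moves it to the height of the BP_FirstPersonCharacter's camera, keeping X and Y.
; Each Tick it looks up the character again and sets the capture's world rotation to half the look-at rotation toward that camera, approximating a reflection angle.
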(event `self.ReceiveBeginPlay`
  (bind _scenecapture (`self.SceneCapture`))
  (bind (_returnvalue_x _returnvalue_y) (`KismetMathLibrary.BreakVector` (`SceneComponent.K2_GetComponentLocation` _scenecapture)))
  (set `self.SceneCapture` (`Actor.GetComponentByClass` (`self.GetOwner`) "/Script/Engine.SceneCaptureComponent2D"))
  ;[1 1 1] Make head height
  (bind _returnvalue (`GameplayStatics.GetActorOfClass` "/Game/FirstPerson/Blueprints/BP_FirstPersonCharacter.BP_FirstPersonCharacter_C"))
  (bind (_returnvalue_x_2 _returnvalue_y_2 _returnvalue_z) (`KismetMathLibrary.BreakVector` (`SceneComponent.K2_GetComponentLocation` (`/Game/FirstPerson/Blueprints/BP_FirstPersonCharacter.FirstPersonCamera` _returnvalue))))
  (`SceneComponent.K2_SetWorldLocation` _scenecapture (`KismetMathLibrary.MakeVector` _returnvalue_x _returnvalue_y _returnvalue_z) false false))

(event `self.ReceiveTick`
  (params (DeltaSeconds :type "Float (single-precision)"))
  (bind _scenecapture (`self.SceneCapture`))
  (bind _returnvalue (`GameplayStatics.GetActorOfClass` "/Game/FirstPerson/Blueprints/BP_FirstPersonCharacter.BP_FirstPersonCharacter_C"))
  (`SceneComponent.K2_SetWorldRotation` _scenecapture (* (`KismetMathLibrary.FindLookAtRotation` (`SceneComponent.K2_GetComponentLocation` _scenecapture) (`SceneComponent.K2_GetComponentLocation` (`/Game/FirstPerson/Blueprints/BP_FirstPersonCharacter.FirstPersonCamera` _returnvalue))) 0.5) false false))